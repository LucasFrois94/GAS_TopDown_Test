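; Gameplay ability for a Leap Slam skill, performed through an animation montage and a gameplay cue.
; On activation it commits cost and builds a GE_Damage spec with set-by-caller damage, though no application of that spec appears here.
; It blocking-loads the montage from the player character's data message and plays it at an attribute-driven rate.
; The cue is removed when the ability ends on montage completion, interruption or cancellation.
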(event `self.K2_ActivateAbility`
  (bind _returnvalue (`GameplayStatics.GetPlayerCharacter` 0))
  (bind (_bsuccessfullyfoundattribute _returnvalue_2) (`AbilitySystemBlueprintLibrary.GetFloatAttribute` _returnvalue (struct :`AttributeName` "AttackSpeed" :`Attribute` "/Script/P_TP_GASTest.PlayerAttributes:AttackSpeed" :`AttributeOwner` "/Script/CoreUObject.Class'/Script/P_TP_GASTest.PlayerAttributes'")))
  (`self.K2_CommitAbilityCost` false)
  (`AbilitySystemBlueprintLibrary.AssignTagSetByCallerMagnitude` (`self.MakeOutgoingGameplayEffectSpec` "/Game/GameplayAbilitySystem/Effects/GE_Damage.GE_Damage_C") (struct :`TagName` "Data.Damage") -15.0)
  (bind _data (message `/Game/GameplayAbilitySystem/BPI_Character.ReturnData` _returnvalue))
  (bind _skill_leapslam (`/Game/GameplayAbilitySystem/Data/DAR_Character.Skill_LeapSlam` _data))
  (`KismetSystemLibrary.LoadAsset_Blocking` _skill_leapslam)
  (if _bsuccessfullyfoundattribute
    (`AbilityTask_PlayMontageAndWait.CreatePlayMontageAndWaitProxy` "None" (`|ConvertAsset` _skill_leapslam) _returnvalue_2
      (:`then`
        (`self.K2_AddGameplayCue` (struct :`TagName` "GameplayCue.LeapSlam"))
        (`KismetSystemLibrary.PrintString` "Ability: Leap Slam"))
      (:`OnCompleted`
        (`self.K2_EndAbility` :!label _label))
      (:`OnInterrupted`
        (goto _label))
      (:`OnCancelled`
        (goto _label)))))

(event `self.K2_OnEndAbility`
  (params (bWasCancelled :type Boolean))
  (`KismetSystemLibrary.PrintString` "Ability Ended"))